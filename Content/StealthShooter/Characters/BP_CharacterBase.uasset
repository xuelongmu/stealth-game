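; Base character Blueprint for the stealth shooter, providing health, death and respawn for combatants.
; On BeginPlay it finds the level's BP_CharacterManager or spawns one, printing a warning if several exist.
; Point damage reduces and prints Health; at zero it calls the empty HandleCharacterDied hook and waits briefly.
; It then asks the manager to respawn the combatant with its controller, detaches and destroys itself.
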(event `self.ReceiveBeginPlay`
  (`self.InitializeCharacterManager`))

(event `self.ReceivePointDamage`
  (params (Damage :type "Float (single-precision)") (DamageType :type "DamageType Object Reference") (HitLocation :type "Vector Structure") (HitNormal :type "Vector Structure") (HitComponent :type "PrimitiveComponent Object Reference") (BoneName :type Name) (ShotFromDirection :type "Vector Structure") (InstigatedBy :type "Controller Object Reference") (DamageCauser :type "Actor Object Reference") (HitInfo :type "HitResult Structure (by ref)"))
  (bind _output_get (set `self.Health` (- (`self.Health`) Damage)))
  (`KismetSystemLibrary.PrintText` (`|FormatText` "Health: {Health}" _output_get))
  (if (<= _output_get 0.0)
    (`self.HandleCharacterDied`)
    (`KismetSystemLibrary.Delay` 2.0)
    (`/Game/StealthShooter/Blueprints/BP_CharacterManager.RespawnCombatant` (`self.CharacterManager`) self (`self.GetController`))
    (`self.DetachFromControllerPendingDestroy`)
    (`self.K2_DestroyActor`)))

(fn `HandleCharacterDied`)

(fn `InitializeCharacterManager`
  (bind _outactors (`GameplayStatics.GetAllActorsOfClass` "/Game/StealthShooter/Blueprints/BP_CharacterManager.BP_CharacterManager_C"))
  (bind _returnvalue (`KismetArrayLibrary.Array_Length` _outactors))
  (if (== _returnvalue 0)
    (bind _returnvalue_2 (`|SpawnActorFromClass` "/Game/StealthShooter/Blueprints/BP_CharacterManager.BP_CharacterManager_C" (`KismetMathLibrary.MakeTransform` (0.0 0.0 0.0)) "AlwaysSpawn" "OverrideRootScale" null null))
    (set `self.CharacterManager` _returnvalue_2)
    (else
      (if (> _returnvalue 1)
        (`KismetSystemLibrary.PrintString` "Too many character managers."))
      (set `self.CharacterManager` (`|GetArrayItem` _outactors)))))

(fn `UserConstructionScript`)