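; BP_CharacterManager handles combatant respawning, giving a controller a new pawn at a random Player Start.
; RespawnCombatant spawns an actor of the supplied combatant's class, casts it to Pawn and has the controller possess it.
; AI controllers are replaced by a newly spawned controller of the same class to reset the behavior tree, while other controllers are reused.
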(fn `RespawnCombatant`
  (params (Type :type "Object Object Reference") (Controller :type "Controller Object Reference"))
  (bind _controller (`self.Controller`))
  (set `self.Controller` Controller)
  (bind _outactors (`GameplayStatics.GetAllActorsOfClass` "/Script/Engine.PlayerStart"))
  (bind _asactor (castclass `Actor` (`GameplayStatics.GetObjectClass` Type)))
  (bind _returnvalue (`|SpawnActorFromClass` _asactor (`KismetMathLibrary.MakeTransform` (.location (`self.GetTransform` (`|GetArrayItem` _outactors (`KismetMathLibrary.RandomInteger` (`KismetArrayLibrary.Array_Length` _outactors))))) (.rotation (`self.GetTransform` (`|GetArrayItem` _outactors (`KismetMathLibrary.RandomInteger` (`KismetArrayLibrary.Array_Length` _outactors)))))) "Undefined" "OverrideRootScale" null null))
  (bind _aspawn (cast `Pawn` _returnvalue))
  (cast `AIController` _controller
    (:`then`
      (bind _asactor_2 (castclass `Actor` (`GameplayStatics.GetObjectClass` _controller)))
      ;[1 1 1] if Controller = AIController, we spawn a brand new AIController so that BT is reset
      (bind _returnvalue_2 (`|SpawnActorFromClass` _asactor_2 (`KismetMathLibrary.MakeTransform` (0.0 0.0 0.0)) "Undefined" "OverrideRootScale" null null))
      (bind _ascontroller (cast `Controller` _returnvalue_2))
      (set `self.Controller` _ascontroller))
    (:`CastFailed`
      _))
  (`Controller.Possess` (`self.Controller`) _aspawn))

(fn `UserConstructionScript`)